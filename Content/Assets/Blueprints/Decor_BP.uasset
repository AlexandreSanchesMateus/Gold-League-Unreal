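; Decor_BP is an actor that moves its Moving component between two relative locations, optionally acting as a one-shot platform.
; After a configurable start delay on BeginPlay, the Move timeline drives a lerp from Loc1 to Loc2.
; When the timeline finishes, the actor destroys itself if DeadPlatform is set, otherwise it replays the motion from the start after a zero-length delay.
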(event `self.ReceiveBeginPlay`
  (`KismetSystemLibrary.Delay` (`self.Delay`))
  (bind (_direction _newtrack_0) (`Timeline|Move` :!label _label)
    (:`Update`
      (`SceneComponent.K2_SetRelativeLocation` (`self.Moving`) (`KismetMathLibrary.VLerp` (`self.Loc1`) (`self.Loc2`) _newtrack_0) false false))
    (:`Finished`
      (if (`self.DeadPlatform`)
        (`self.K2_DestroyActor`)
        (else
          (`KismetSystemLibrary.Delay` 0.0)
          (goto _label :!via `PlayFromStart`))))))

(fn `UserConstructionScript`)