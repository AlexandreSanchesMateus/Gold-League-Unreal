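; Enemy AI character that shoots at the player, reacts to point damage and ragdolls on death.
; BeginPlay seeds the Blackboard with player and spawn location; StartFire/StopFire control a looping timer that line-traces toward the player to apply damage.
; Hits reduce health, spawn blood particles and play a reaction montage, or at zero health stop AI logic and push the struck bone.
; BloodSplatter traces behind hits but only prints debug text; its decal spawn is disconnected.
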(event `self.ReceiveBeginPlay`
  (bind _returnvalue (`AIBlueprintHelperLibrary.GetBlackboard` null))
  ;[1 1 1] begin play
  (`BlackboardComponent.SetValueAsObject` _returnvalue "Enemy" (`GameplayStatics.GetPlayerCharacter` 0))
  (`BlackboardComponent.SetValueAsVector` _returnvalue "DefaultLocation" (`self.K2_GetActorLocation` self)))

(event `self.ReceivePointDamage`
  (params (Damage :type "Float (single-precision)") (DamageType :type "DamageType Object Reference") (HitLocation :type "Vector Structure") (HitNormal :type "Vector Structure") (HitComponent :type "PrimitiveComponent Object Reference") (BoneName :type Name) (ShotFromDirection :type "Vector Structure") (InstigatedBy :type "Controller Object Reference") (DamageCauser :type "Actor Object Reference") (HitInfo :type "HitResult Structure (by ref)"))
  (bind (_bblockinghit _binitialoverlap _time _distance _location _impactpoint _normal _impactnormal _physmat _hitactor _hitcomponent _hitbonename) (`GameplayStatics.BreakHitResult` HitInfo))
  (bind _health (`self.Health`))
  ;[1 1 1] Take damage
  (set `self.Health` (- _health Damage))
  (if (<= _health 0.0)
    (`self.On Death` ShotFromDirection (`self.DeathForce`) _hitbonename)
    (else
      (`|PlayMontage` (`self.Mesh`) "/Game/IA-Enemy/Animation/With-Rifle/Montage/Hit_Reaction__Montage.Hit_Reaction__Montage"
        (:`then`
          _))))
  (`self.Blood Splatter` _location (+ _location (* ShotFromDirection 200.0)))
  (`GameplayStatics.SpawnEmitterAtLocation` "/Game/Import/P_Blood.P_Blood" _location (`KismetMathLibrary.MakeRotFromX` _normal) (2.0 2.0 2.0)))

(event `Start Fire`
  ;[1 1 1] Fite système
  (bind _returnvalue (`KismetSystemLibrary.K2_SetTimerDelegate` (delegate `Fire`) 1.0 true))
  (set `self.TimerHandle` _returnvalue))

(event `Stop Fire`
  (bind _timerhandle (`self.TimerHandle`))
  ;[1 1 1] Fite système
  (if (`KismetSystemLibrary.K2_IsValidTimerHandle` _timerhandle)
    (`KismetSystemLibrary.K2_ClearAndInvalidateTimerHandle` _timerhandle)))

(event `Fire`
  (bind _returnvalue (`SceneComponent.K2_GetComponentLocation` (`self.FirePoint`)))
  ;[1 1 1] Fite système
  (bind (_outhit _returnvalue_2) (`KismetSystemLibrary.LineTraceSingleByProfile` :`Start` _returnvalue :`End` (+ _returnvalue (* (- (`self.K2_GetActorLocation` (`GameplayStatics.GetPlayerCharacter` 0)) _returnvalue) 100.0)) :`DrawDebugType` "ForDuration" :`DrawTime` 1.0))
  (if _returnvalue_2
    (bind _asfirst_person_character (cast `/Game/FirstPersonCPP/Blueprints/FirstPersonCharacter` (`.HitActor` (`GameplayStatics.BreakHitResult` _outhit))))
    (`GameplayStatics.ApplyDamage` _asfirst_person_character 10.0)))

(fn `Blood Splatter`
  (params (Start :type "Vector Structure") (End :type "Vector Structure"))
  (returns (SpawnDecal :type Boolean))
  (bind (_outhit _returnvalue) (`KismetSystemLibrary.LineTraceSingle` :`Start` Start :`End` End :`TraceChannel` "TraceTypeQuery1" :`DrawDebugType` "ForDuration" :`TraceColor` (struct :`R` 0.107652 :`B` 1.0 :`A` 1.0) :`DrawTime` 10.0))
  (if _returnvalue
    (if (`|EnumEquality` (`SceneComponent.Mobility` (`.HitComponent` (`GameplayStatics.BreakHitResult` _outhit))) "Static")
      (`KismetSystemLibrary.PrintString` "yes")
      (else
        (`KismetSystemLibrary.PrintString` "false")))))

(fn `On Death`
  (params (LastHitFrom :type "Vector Structure") (Force :type "Float (double-precision)") (Bone :type Name))
  (bind _mesh (`self.Mesh`))
  (`|ExecutionSequence`
    (:`then_0`
      (`self.Stop Fire`)
      (`BrainComponent.StopLogic` (`AIController.BrainComponent` (`AIBlueprintHelperLibrary.GetAIController` self)) "Dead"))
    (:`then_1`
      ;[1 1 1] Ragdoll
      (`PrimitiveComponent.SetSimulatePhysics` _mesh true)
      (`PrimitiveComponent.SetCollisionProfileName` _mesh "Ragdoll" true)
      (`PrimitiveComponent.SetCollisionEnabled` (`self.CapsuleComponent`) "NoCollision")
      (`PrimitiveComponent.AddForce` _mesh (* LastHitFrom Force) Bone false))))

(fn `UserConstructionScript`)