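; Behavior tree task that picks a cover point for an enemy AI, hidden from its current Enemy target.
; It clears IsInCover, then line-traces from each of the pawn's Cover actors to the player's camera, rejecting those that hit a Character.
; The nearest unoccupied remaining cover, by squared distance, is written to a configurable blackboard key.
; It fails only when the Cover list is empty, and traces draw debug lines.
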(event `self.ReceiveExecuteAI`
  (params (OwnerController :type "AIController Object Reference") (ControlledPawn :type "Pawn Object Reference"))
  (bind _returnvalue (`AIBlueprintHelperLibrary.GetBlackboard` ControlledPawn))
  ;[1 1 1] Anti camarabe bouré
  (bind _asbp_ia_enemy (cast `/Game/IA-Enemy/Blueprint/BP_IA-Enemy` ControlledPawn))
  (bind _cover (`/Game/IA-Enemy/Blueprint/BP_IA-Enemy.Cover` _asbp_ia_enemy))
  (if (> (`KismetArrayLibrary.Array_Length` _cover) 0)
    ;[1 1 1] Initialisation
    (set `self.BestCoverDistance` 9000000.0)
    (`BlackboardComponent.SetValueAsBool` _returnvalue "IsInCover" false)
    ;[1 1 1] Iteration sur chaque position : si il est en face du joueur & le plus proche de l'IA
    (for _array_element _cover
      (bind _returnvalue_2 (`Actor.K2_GetActorLocation` _array_element))
      (bind _outhit (`KismetSystemLibrary.LineTraceSingleByProfile` _returnvalue_2 (`SceneComponent.K2_GetComponentLocation` (`Gold_League_ProjectCharacter.FirstPersonCameraComponent` (cast `/Game/FirstPersonCPP/Blueprints/FirstPersonCharacter` (`BlackboardComponent.GetValueAsObject` _returnvalue "Enemy") :!pure true))) "None" false (`|MakeArray` ControlledPawn :!type "Actor Object Reference") "ForDuration" true (struct :`R` 0.090804 :`G` 1.0 :`A` 1.0) (struct :`R` 1.0 :`B` 0.006983 :`A` 1.0)))
      (cast `Character` (`.HitActor` (`GameplayStatics.BreakHitResult` _outhit))
        (:`CastFailed`
          (bind _returnvalue_3 (`KismetMathLibrary.Vector_DistanceSquared` _returnvalue_2 (`Actor.K2_GetActorLocation` ControlledPawn)))
          (if (and (not (`/Game/IA-Enemy/Blueprint/Cover_Actor_Blueprint.IsOccupied` (cast `/Game/IA-Enemy/Blueprint/Cover_Actor_Blueprint` _array_element :!pure true))) (< _returnvalue_3 (`self.BestCoverDistance`)))
            (set `self.BestCoverDistance` _returnvalue_3)
            (set `self.BestCover` _array_element)))))
    (`BlackboardComponent.SetValueAsObject` _returnvalue (`self.Key Name`) (`self.BestCover`))
    (`self.FinishExecute` true)
    (else
      (`self.FinishExecute` false))))