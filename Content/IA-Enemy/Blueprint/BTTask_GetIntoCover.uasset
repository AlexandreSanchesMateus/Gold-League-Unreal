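; Behavior tree task that sends an IA enemy into the cover actor stored in its blackboard.
; It reads the cover key, moves the AI to that actor's location, then on arrival calls EnterCover on the enemy and sets the cover bool key to true.
; A failed move request finishes the task as failed, while a finished move reports success.
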(event `self.ReceiveExecuteAI`
  (params (OwnerController :type "AIController Object Reference") (ControlledPawn :type "Pawn Object Reference"))
  (bind _returnvalue (`AIBlueprintHelperLibrary.GetBlackboard` ControlledPawn))
  (bind _asactor (cast `Actor` (`BlackboardComponent.GetValueAsObject` _returnvalue (`self.BB_Cover`))))
  (`AITask_MoveTo.AIMoveTo` OwnerController (`Actor.K2_GetActorLocation` _asactor) null
    (:`OnRequestFailed`
      (`self.FinishExecute` false))
    (:`OnMoveFinished`
      (bind _asbp_ia_enemy (cast `/Game/IA-Enemy/Blueprint/BP_IA-Enemy` ControlledPawn))
      (`/Game/IA-Enemy/Blueprint/BP_IA-Enemy.Enter Cover` _asbp_ia_enemy)
      (`BlackboardComponent.SetValueAsBool` _returnvalue (`self.BB_CoverBool`) true)
      (`self.FinishExecute` true))))