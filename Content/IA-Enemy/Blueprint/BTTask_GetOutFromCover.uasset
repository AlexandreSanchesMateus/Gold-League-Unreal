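; Behavior tree task that brings a BP_IA-Enemy out of cover.
; It uncrouches the enemy, then reads the cover actor from the blackboard's CoverActor key.
; Crouch-height cover finishes the task at once; other cover plays a right or left emerge montage based on the cover's EmergeRight flag.
; The task reports success as soon as the montage starts, without waiting for it to end.
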(event `self.ReceiveExecuteAI`
  (params (OwnerController :type "AIController Object Reference") (ControlledPawn :type "Pawn Object Reference"))
  (bind _asbp_ia_enemy (cast `/Game/IA-Enemy/Blueprint/BP_IA-Enemy` ControlledPawn))
  (`|ExecutionSequence`
    (:`then_0`
      (if (`NavMovementComponent.IsCrouching` (`Character.CharacterMovement` _asbp_ia_enemy))
        (`Character.UnCrouch` _asbp_ia_enemy)))
    (:`then_1`
      (bind _ascover_actor_blueprint (cast `/Game/IA-Enemy/Blueprint/Cover_Actor_Blueprint` (`BlackboardComponent.GetValueAsObject` (`AIBlueprintHelperLibrary.GetBlackboard` ControlledPawn) "CoverActor")))
      (if (`/Game/IA-Enemy/Blueprint/Cover_Actor_Blueprint.NeedCrouch` _ascover_actor_blueprint)
        (`self.FinishExecute` true)
        (else
          (if (`/Game/IA-Enemy/Blueprint/Cover_Actor_Blueprint.emergeRight` _ascover_actor_blueprint)
            (bind _mesh (`Character.Mesh` _asbp_ia_enemy))
            (`|PlayMontage` _mesh "/Game/IA-Enemy/Animation/With-Rifle/Montage/Emerging_Right_2_Montage.Emerging_Right_2_Montage"
              (:`then`
                (`KismetSystemLibrary.PrintString` "Right")))
            (else
              (`|PlayMontage` _mesh "/Game/IA-Enemy/Animation/With-Rifle/Montage/Emerging_Left_Montage.Emerging_Left_Montage"
                (:`then`
                  (`KismetSystemLibrary.PrintString` "Left")))))
          (`self.FinishExecute` true))))))