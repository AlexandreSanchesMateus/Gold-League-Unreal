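; Behavior tree task for enemy AI that checks whether its current cover is exposed to the player.
; It line-traces from the blackboard CoverActor to the player's first-person camera, ignoring the controlled pawn and drawing debug lines.
; A hit on the player clears IsInCover and succeeds, so success means invalid cover; any other result fails.
; A missing CoverActor leaves the task unfinished.
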(event `self.ReceiveExecuteAI`
  (params (OwnerController :type "AIController Object Reference") (ControlledPawn :type "Pawn Object Reference"))
  (bind _returnvalue (`AIBlueprintHelperLibrary.GetBlackboard` ControlledPawn))
  (bind _asactor (cast `Actor` (`BlackboardComponent.GetValueAsObject` _returnvalue "CoverActor")))
  (bind _outhit (`KismetSystemLibrary.LineTraceSingleByProfile` (`Actor.K2_GetActorLocation` _asactor) (`SceneComponent.K2_GetComponentLocation` (`Gold_League_ProjectCharacter.FirstPersonCameraComponent` (cast `/Game/FirstPersonCPP/Blueprints/FirstPersonCharacter` (`GameplayStatics.GetPlayerCharacter` 0) :!pure true))) "None" false (`|MakeArray` ControlledPawn :!type "Actor Object Reference") "ForDuration" true (struct :`G` 1.0 :`B` 0.067879 :`A` 1.0) (struct :`R` 1.0 :`A` 1.0)))
  (cast `/Game/FirstPersonCPP/Blueprints/FirstPersonCharacter` (`.HitActor` (`GameplayStatics.BreakHitResult` _outhit))
    (:`then`
      (`BlackboardComponent.SetValueAsBool` _returnvalue "IsInCover" false)
      (`self.FinishExecute` true))
    (:`CastFailed`
      (`self.FinishExecute` false))))