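; Behavior Tree task that randomly decides whether an enemy AI flanks.
; On execute it clears the IsInCover blackboard key, then compares the ProbFlank variable against a random integer roll on a percentage scale.
; A passing roll finishes the task successfully, while a failing one also clears AlertState and finishes as failed.
; Both outcomes print a debug string.
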(event `self.ReceiveExecuteAI`
  (params (OwnerController :type "AIController Object Reference") (ControlledPawn :type "Pawn Object Reference"))
  (bind _returnvalue (`AIBlueprintHelperLibrary.GetBlackboard` ControlledPawn))
  (`BlackboardComponent.SetValueAsBool` _returnvalue "IsInCover" false)
  (if (>= (`self.ProbFlank`) (`KismetMathLibrary.RandomIntegerInRange` 0 100))
    (`KismetSystemLibrary.PrintString` "Flank")
    (`self.FinishExecute` true)
    (else
      (`BlackboardComponent.SetValueAsBool` _returnvalue "AlertState" false)
      (`KismetSystemLibrary.PrintString` "Abord")
      (`self.FinishExecute` false))))