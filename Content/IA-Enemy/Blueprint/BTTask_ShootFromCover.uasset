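; Behavior tree task for the enemy AI that leaves cover by clearing the IsInCover blackboard flag; despite its name, it contains no shooting logic.
; A Sequence issues AI moves to DefaultLocation and MoveLocation back to back, without waiting between them.
; The first move ends in an unconnected delay, while finishing the second clears AlertState and completes the task.
; The UnCrouch call is disconnected, leaving only an "Uncrouch" debug print.
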(event `self.ReceiveExecuteAI`
  (params (OwnerController :type "AIController Object Reference") (ControlledPawn :type "Pawn Object Reference"))
  (bind _returnvalue (`AIBlueprintHelperLibrary.GetBlackboard` ControlledPawn))
  (bind _asbp_ia_enemy (cast `/Game/IA-Enemy/Blueprint/BP_IA-Enemy` ControlledPawn))
  (`KismetSystemLibrary.PrintString` "Uncrouch")
  (`BlackboardComponent.SetValueAsBool` _returnvalue "IsInCover" false)
  (`|ExecutionSequence`
    (:`then_0`
      (`AITask_MoveTo.AIMoveTo` OwnerController (`BlackboardComponent.GetValueAsVector` _returnvalue "DefaultLocation") null
        (:`OnMoveFinished`
          (`KismetSystemLibrary.Delay` 3.0))))
    (:`then_1`
      (`AITask_MoveTo.AIMoveTo` OwnerController (`BlackboardComponent.GetValueAsVector` _returnvalue "MoveLocation") null
        (:`OnMoveFinished`
          (`BlackboardComponent.SetValueAsBool` _returnvalue "AlertState" false)
          (`self.FinishExecute` true))))))