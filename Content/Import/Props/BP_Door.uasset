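; BP_Door is a hinged door prop that toggles open and closed through its OpenDoor event.
; A dot product between the player-to-door direction and the door's forward vector picks which way it swings, based on the player's side.
; The OpenClose timeline lerps the Pivot's yaw up to a quarter turn.
; Later calls reverse the timeline, and finishing backward marks the door closed again.
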(event `self.ReceiveBeginPlay`
  ;[1 1 1] Get Player Ref
  (bind _asfirst_person_character (cast `/Game/FirstPersonCPP/Blueprints/FirstPersonCharacter` (`GameplayStatics.GetPlayerCharacter` 0)))
  (set `self.Player` _asfirst_person_character))

(event `OpenDoor`
  (bind _defaultsceneroot (`self.DefaultSceneRoot`))
  ;[1 1 1] Open/Close
  (if (`self.isDoorClosed`)
    (set `self.isDoorClosed` false)
    (set `self.Dot` (`KismetMathLibrary.Dot_VectorVector` (`KismetMathLibrary.Normal` (- (`SceneComponent.K2_GetComponentLocation` _defaultsceneroot) (`self.K2_GetActorLocation` (`self.Player`)))) (`SceneComponent.GetForwardVector` _defaultsceneroot)))
    (bind (_direction _alpha) (`Timeline|Open/Close` :!label _label)
      (:`Update`
        (`SceneComponent.K2_SetRelativeRotation` (`self.Pivot`) (`KismetMathLibrary.MakeRotator` 0.0 0.0 (`KismetMathLibrary.Lerp` 0.0 (`KismetMathLibrary.SelectFloat` 90.0 -90.0 (>= (`self.Dot`) 0.0)) _alpha)) false false))
      (:`Finished`
        (switch `ETimelineDirection` _direction
          (:`Backward`
            (set `self.isDoorClosed` true)))))
    (else
      (goto _label :!via `Reverse`))))

(fn `UserConstructionScript`)